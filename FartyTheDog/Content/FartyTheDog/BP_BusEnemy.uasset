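; BP_BusEnemy is an enemy in Farty the Dog that patrols back and forth along the world X axis.
; Each Tick it applies half-strength movement input in the current direction while a step counter counts up to a fixed limit or back down to zero.
; At either end it flips the WalkingRight flag to reverse.
; The range is counted in frames rather than distance, so patrol length depends on frame rate.
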(event EventBeginPlay
  (Variables|Default|SetMaxMoveLateral 2e+02)
  (Variables|Default|SetMoveLateral 0.0)
  (Variables|Default|SetwalkingRight true))

(event Collision|EventActorBeginOverlap
  (params (OtherActor :type Actor%20Object%20Reference)))

(event EventTick
  (params (DeltaSeconds :type Float%20%28single-precision%29))
  (if (Variables|Default|GetwalkingRight)
    (if (> (Variables|Default|GetMaxMoveLateral) (Variables|Default|GetMoveLateral))
      (Pawn|Input|AddMovementInput "1.000000,0.000000,0.000000" 0.5 false)
      (Variables|Default|SetwalkingRight true)
      (Math|Float|IncrementFloat (Variables|Default|GetMoveLateral))
      (else
        (Variables|Default|SetwalkingRight false)))
    (elif (> (Variables|Default|GetMoveLateral) 0.0)
      (Pawn|Input|AddMovementInput "-1.000000,0.000000,0.000000" 0.5 false)
      (Variables|Default|SetwalkingRight false)
      (Math|Float|DecrementFloat (Variables|Default|GetMoveLateral))
      (else
        (Variables|Default|SetwalkingRight true)))))

(fn ConstructionScript)