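; Police officer enemy character for FartyTheDog that chases the player and plays an attack animation when close.
; PawnSensing sightings trigger FollowPlayer, which uses AI MoveTo toward player 0 and plays the attack montage on arrival.
; A CanAttack flag with a montage-length delay gates attacks, but every sighting resets it.
; The seen flag is never effectively cleared, the stop-movement logic is unconnected, and no damage is applied here.
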(event OnSeePawn(PawnSensing)
  (params (Pawn :type Pawn%20Object%20Reference))
  (Variables|Default|SetisSeingPlayer true)
  (CallFunction|FollowPlayer))

(event Custom|FollowPlayer
  (Variables|Default|SetcanAttack true)
  (if (Variables|Default|GetisSeingPlayer)
    (AI|AIMoveTo self "0, 0, 0" (Game|GetPlayerCharacter 0) 4e+02 false
      (:OnSuccess
        (if (Variables|Default|GetcanAttack)
          (Variables|Default|SetcanAttack false)
          (bind _returnvalue (Animation|PlayAnimMontage "/Game/Characters/Police/A_Police_Attack_Montage.A_Police_Attack_Montage" 1.0 "None"))
          (Utilities|FlowControl|Delay _returnvalue)
          (Variables|Default|SetcanAttack true)
          (Development|PrintString "can attack again"))))
    (else
      (Variables|Default|SetisSeingPlayer false))))

(event EventBeginPlay
  (|CallParentFunction) ; This node is disabled and will not be called.\nDrag off pins to build functionality.
)

(event Collision|EventActorBeginOverlap
  (params (OtherActor :type Actor%20Object%20Reference))
  (|CallParentFunction OtherActor) ; This node is disabled and will not be called.\nDrag off pins to build functionality.
)

(event EventTick
  (params (DeltaSeconds :type Float%20%28single-precision%29))
  (|CallParentFunction DeltaSeconds))

(fn ConstructionScript
  (|CallParentFunction))