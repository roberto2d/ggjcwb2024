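; BP_PoliceEnemy is a police enemy in the FartyTheDog game, currently with no active movement behavior.
; BeginPlay only resets its lateral patrol counter, limit and direction flag, while Tick and overlap are empty.
; Two disconnected chains never run: a left-right patrol along X using a step counter and AddMovementInput, and a SimpleMoveToActor chase of the player character.
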(event EventBeginPlay
  (Variables|Default|SetMaxMoveLateral 0.0)
  (Variables|Default|SetMoveLateral 0.0)
  (Variables|Default|SetwalkingRight true))

(event Collision|EventActorBeginOverlap
  (params (OtherActor :type Actor%20Object%20Reference)))

(event EventTick
  (params (DeltaSeconds :type Float%20%28single-precision%29)))

(fn ConstructionScript)